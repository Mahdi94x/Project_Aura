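; Gameplay ability for a melee attack against the avatar's combat target.
; It updates the motion-warp facing toward the target, plays a random tagged attack montage and waits for that montage's gameplay event.
; On the event, it finds live characters around the montage's combat socket, damages non-friends and calls EndAbility on any friend found.
; A hit fires the MeleeImpact gameplay cue, and the ability ends after the check or montage completion or interruption.
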(event Ability|EventActivateAbility
  (bind _returnvalue (Ability|GetAvatarActorfromActorInfo))
  (bind _returnvalue_2 (Ability|GetAvatarActorfromActorInfo))
  (Variables|Default|SetHasHitTarget false)
  (bind _returnvalue_3 (Class|EnemyHighlightInterface|GetCombatTarget(Message) _returnvalue))
  (bind _output_get (Variables|Default|SetCombatTarget _returnvalue_3))
  (Class|CombatInterface|UpdateFacingWarpTarget(Message) _returnvalue (Transformation|GetActorLocation _output_get))
  (bind _returnvalue_4 (Class|CombatInterface|GetAttackTaggedMontages(Message) _returnvalue))
  (bind _output_get_2 (Variables|Default|SetTaggedMontage (Class|AuraBaseDamageAbility|GetRandomTaggedMontagefromArray _returnvalue_4)))
  (|PlayMontageandWaitProxy "None" (.Montage (Utilities|Struct|BreakTaggedMontage _output_get_2)) 1.0 "None" false 1.0 0.0 false
    (:then
      (Ability|Tasks|WaitGameplayEvent (.MontageTag (Utilities|Struct|BreakTaggedMontage _output_get_2)) 0 true
        (:EventReceived
          (bind _returnvalue_5 (Class|CombatInterface|GetCombatSocketLocation(Message) _returnvalue_2 (.SocketTag (Utilities|Struct|BreakTaggedMontage _output_get_2))))
          (Variables|Default|SetCombatSocketLocation _returnvalue_5)
          (bind _returnvalue_6 (Class|EnemyHighlightInterface|GetSphereTraceRadius(Message) _returnvalue_2))
          (bind _outoverlappingactors (Class|AuraAbilitySystemLibrary|GetLivePlayersWithinRadius _returnvalue_2 (Utilities|Array|MakeArray _returnvalue_2) _returnvalue_6 (Variables|Default|GetCombatSocketLocation)))
          (for _array_element _outoverlappingactors
            (bind _output_get_3 (Variables|Default|SetAliveTargetElement _array_element))
            (if (Class|AuraAbilitySystemLibrary|IsNotFriend (Ability|GetAvatarActorfromActorInfo) _array_element)
              (Class|AuraBaseDamageAbility|CauseDamageMelee _output_get_3)
              (Variables|Default|SetHasHitTarget true)
              (else
                (Ability|EndAbility))))
          (if (Variables|Default|GetHasHitTarget)
            (Class|GameplayAbility|ExecuteGameplayCuewithParams "(TagName=\"GameplayCue.MeleeImpact\")" (Ability|GameplayCue|MakeGameplayCueParameters :AggregatedSourceTags (GameplayTags|MakeGameplayTagContainerfromTag (.MontageTag (Utilities|Struct|BreakTaggedMontage (Variables|Default|GetTaggedMontage)))) :Location (Variables|Default|GetCombatSocketLocation) :EffectCauser (Ability|GetAvatarActorfromActorInfo) :SourceObject (Variables|Default|GetCombatTarget))))
          (Ability|EndAbility))))
    (:OnCompleted
      (Ability|EndAbility :!label _label))
    (:OnInterrupted
      (goto _label))
    (:OnCancelled
      (goto _label))))

(event Ability|EventOnEndAbility
  (params (bWasCancelled :type Boolean)))