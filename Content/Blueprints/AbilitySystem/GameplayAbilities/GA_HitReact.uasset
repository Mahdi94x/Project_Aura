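; GA_HitReact is a gameplay ability that plays a hit reaction on its avatar.
; On activation it applies GE_HitReact to the owner and stores the handle, then plays the montage returned by the avatar's CombatInterface.
; When the montage completes, is interrupted or is cancelled, it removes the effect by that handle and ends.
; If the interface cast fails, it logs and ends without removing the effect.
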(event Ability|EventActivateAbility
  (bind _returnvalue (Ability|ApplyGameplayEffectToOwner "/Game/Blueprints/AbilitySystem/GameplayEffect/GE_HitReact.GE_HitReact_C"))
  (Variables|Default|SetActive%20GE%20HitReact%20Handle _returnvalue)
  (bind _ascombat_interface (Utilities|Casting|CastToCombatInterface (Ability|GetAvatarActorfromActorInfo))
    (:then
      (bind _returnvalue_2 (Class|CombatInterface|GetHitReactMontage _ascombat_interface))
      (|PlayMontageandWaitProxy "None" _returnvalue_2 1.0 "None" true 1.0 0.0 false
        (:OnCompleted
          _)
        (:OnInterrupted
          _)
        (:OnCancelled
          _))
      (Ability|RemoveGameplayEffectFromOwnerWithHandle (Variables|Default|GetActive%20GE%20HitReact%20Handle))
      (Ability|EndAbility))
    (:CastFailed
      (Development|PrintString "Failed to retreive the montage - EndAbility" true true "(R=0.000000,G=0.660000,B=1.000000,A=1.000000)" 5.0)
      (Ability|EndAbility))))

(event Ability|EventOnEndAbility
  (params (bWasCancelled :type Boolean)))