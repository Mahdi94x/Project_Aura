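; Ranged attack gameplay ability that fires a projectile at the avatar's combat target.
; On activation it feeds the target's location to the avatar's facing motion-warp update and plays the avatar's first tagged attack montage.
; The montage's gameplay event triggers SpawnProjectile from the tagged socket toward that cached location, with optional pitch override.
; The ability then ends without stopping the montage, or ends when the montage completes or is interrupted.
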(event Ability|EventActivateAbility
  (bind _returnvalue (Ability|GetAvatarActorfromActorInfo))
  (bind _returnvalue_2 (Class|EnemyHighlightInterface|GetCombatTarget(Message) (Ability|GetAvatarActorfromActorInfo)))
  (bind _output_get (Variables|Default|SetCombatTarget _returnvalue_2))
  (bind _output_get_2 (Variables|Default|SetCombatTargetLocation (Transformation|GetActorLocation _output_get)))
  (Class|CombatInterface|UpdateFacingWarpTarget(Message) _returnvalue _output_get_2)
  (bind _returnvalue_3 (Class|CombatInterface|GetAttackTaggedMontages(Message) _returnvalue))
  (bind _output_get_3 (Variables|Default|SetTaggedMontage (Utilities|Array|Get(acopy) _returnvalue_3)))
  (|PlayMontageandWaitProxy "None" (.Montage (Utilities|Struct|BreakTaggedMontage _output_get_3)) 1.0 "None" false 1.0 0.0 false
    (:then
      (Ability|Tasks|WaitGameplayEvent (.MontageTag (Utilities|Struct|BreakTaggedMontage _output_get_3)) 0 true
        (:EventReceived
          (Class|AuraProjectileSpellGA|SpawnProjectile (Variables|Default|GetCombatTargetLocation) (.SocketTag (Utilities|Struct|BreakTaggedMontage _output_get_3)) (Variables|Default|GetOverride%20Pitch) (Variables|Default|GetPitch%20Override))
          (Ability|EndAbility))))
    (:OnCompleted
      (Ability|EndAbility :!label _label))
    (:OnInterrupted
      (goto _label))
    (:OnCancelled
      (goto _label))))

(event Ability|EventOnEndAbility
  (params (bWasCancelled :type Boolean)))