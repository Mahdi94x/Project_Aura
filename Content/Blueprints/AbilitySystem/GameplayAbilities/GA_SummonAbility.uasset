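; Gameplay ability that summons random minions around the casting avatar, using a montage tagged for summon attacks.
; On activation it shuffles the spawn locations, plays a ground-summon Niagara effect at each, then starts the montage.
; The montage's gameplay event triggers a delayed, index-driven loop that spawns AI-controlled minions one by one, slightly raised and facing away from the caster.
; The ability ends once every location is used.
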(event Ability|EventActivateAbility
  (bind _returnvalue (Class|CombatInterface|GetTaggedMontagebyTag(Message) (Ability|GetAvatarActorfromActorInfo) (GameplayTags|MakeLiteralGameplayTag "(TagName=\"Montage.Attack.Summon\")")))
  (Variables|Default|SetSummonMontage _returnvalue)
  (bind _returnvalue_2 (Class|AuraSummonAbility|GetSpawnLocations))
  (bind _output_get (Variables|Default|SetSpawnLocations _returnvalue_2))
  (Utilities|Array|Shuffle _output_get)
  (for _array_element (Variables|Default|GetSpawnLocations)
    (Niagara|SpawnSystematLocation "/Game/Assets/Effects/Combat/NS_GroundSummon.NS_GroundSummon" _array_element))
  (|PlayMontageandWaitProxy "None" (.Montage (Utilities|Struct|BreakTaggedMontage (Variables|Default|GetSummonMontage))) 1.0 "None" true 1.0 0.0 false
    (:then
      (Ability|Tasks|WaitGameplayEvent (.MontageTag (Utilities|Struct|BreakTaggedMontage (Variables|Default|GetSummonMontage))) 0
        (:EventReceived
          (Utilities|FlowControl|Delay 0.5)
          (if (CallFunction|CheckArrayBounds) :!label _label
            (bind _returnvalue_3 (Game|SpawnActorfromClass (Class|AuraSummonAbility|GetRandomMiniontoSpawn) (Math|Transform|MakeTransform (+ (Utilities|Array|Get(acopy) (Variables|Default|GetSpawnLocations) (Variables|Default|GetSpawnLocationIndex)) "0.000000,0.000000,70.000000") (Math|Rotator|FindLookatRotation (Transformation|GetActorLocation (Ability|GetAvatarActorfromActorInfo)) (+ (Utilities|Array|Get(acopy) (Variables|Default|GetSpawnLocations) (Variables|Default|GetSpawnLocationIndex)) "0.000000,0.000000,70.000000")) "1.000000,1.000000,1.000000") "AlwaysSpawn" "MultiplyWithRoot" 0 0))
            (Pawn|SpawnDefaultController _returnvalue_3)
            (Math|Integer|IncrementInt (Variables|Default|GetSpawnLocationIndex)
              (:%20%20
                (Utilities|FlowControl|Delay 0.2)
                (goto _label)))
            (else
              (Ability|EndAbility))))))))

(event Ability|EventOnEndAbility
  (params (bWasCancelled :type Boolean)))

(fn CheckArrayBounds
  (return (< (Variables|Default|GetSpawnLocationIndex) (Utilities|Array|Length (Variables|Default|GetSpawnLocations)))))

(fn NewFunction
  (if (CallFunction|CheckArrayBounds)
    (Rendering|Debug|DrawDebugSphere (Utilities|Array|Get(acopy) (Variables|Default|GetSpawnLocations) (Variables|Default|GetSpawnLocationIndex)) 2e+01 12 "(R=1.000000,G=0.056416,B=0.741145,A=1.000000)" 3.0)
    (Math|Integer|IncrementInt (Variables|Default|GetSpawnLocationIndex))))