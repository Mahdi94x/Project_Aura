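; BP_Demon_Base is a demon enemy base Blueprint that animates the mesh scale when the demon spawns.
; On BeginPlay it calls the parent, then plays SpawnTimeline, whose ScaleTrack drives a uniform relative scale on the Mesh while it is valid.
; All other behavior is left to the parent class, as Tick and overlap events are disabled and the construction script only calls its parent.
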(event EventBeginPlay
  (|CallParentFunction)
  (bind _scaletrack (Timeline|SpawnTimeline Play)
    (:Update
      (bind _mesh (Variables|Character|GetMesh)
        (:then
          (Transformation|SetRelativeScale3D _mesh (Math|Vector|MakeVector _scaletrack _scaletrack _scaletrack)))
        (:else)))))

(event Collision|EventActorBeginOverlap
  (params (OtherActor :type Actor%20Object%20Reference))
  (|CallParentFunction OtherActor) ; This node is disabled and will not be called.\nDrag off pins to build functionality.
)

(event EventTick
  (params (DeltaSeconds :type Float%20%28single-precision%29))
  (|CallParentFunction DeltaSeconds) ; This node is disabled and will not be called.\nDrag off pins to build functionality.
)

(fn ConstructionScript
  (|CallParentFunction))