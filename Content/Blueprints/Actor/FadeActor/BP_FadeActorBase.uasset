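; Base actor that fades its mesh out and back in through a timeline-driven material parameter.
; The construction script caches the original materials and builds dynamic instances from a separate set of fade materials.
; FadeOut swaps in those instances and plays the timeline on their Fade parameter, while Fadein reverses it.
; At full Fade the original materials return and Visibility blocking is optionally restored; at zero the mesh ignores that channel.
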(event EventBeginPlay)

(event EventFadein
  (bind _fade (Timeline|FadeTimeline Reverse)
    (:Update
      (for _array_element (Variables|Default|GetDynamicFadeMatInst)
        (Rendering|Material|SetScalarParameterValue _array_element "Fade" _fade :!class /Script/Engine.MaterialInstanceDynamic)))
    (:Finished
      (CallFunction|FadeFinished _fade))))

(event EventFadeOut
  (CallFunction|SetMaterialtoDynamicInstances)
  (bind _fade (Timeline|FadeTimeline Play)
    (:Update
      (for _array_element (Variables|Default|GetDynamicFadeMatInst)
        (Rendering|Material|SetScalarParameterValue _array_element "Fade" _fade :!class /Script/Engine.MaterialInstanceDynamic)))
    (:Finished
      (CallFunction|FadeFinished _fade))))

(fn ConstructionScript
  (Utilities|Array|Clear (Variables|Default|GetDynamicFadeMatInst))
  (Variables|Default|SetOriginalMaterials (Rendering|Material|GetMaterials (Variables|Default|GetMesh)))
  (for _array_element (Variables|Default|GetFadeMaterialsInst)
    (bind _returnvalue (Rendering|Material|CreateDynamicMaterialInstance _array_element "None" "None" :!class /Script/Engine.KismetMaterialLibrary))
    (Utilities|Array|AddUnique (Variables|Default|GetDynamicFadeMatInst) _returnvalue)))

(fn SetMaterialtoDynamicInstances
  (for (_array_element _array_index) (Variables|Default|GetDynamicFadeMatInst)
    (Rendering|Material|SetMaterial (Variables|Default|GetMesh) _array_index _array_element)))

(fn ResetMaterialstoOriginal
  (for (_array_element _array_index) (Variables|Default|GetOriginalMaterials)
    (Rendering|Material|SetMaterial (Variables|Default|GetMesh) _array_index _array_element)))

(fn FadeFinished
  (params (Fade :type Float%20%28single-precision%29))
  (if (>= Fade 1.0)
    (CallFunction|ResetMaterialstoOriginal)
    (if (Variables|Default|GetBlockVisibility)
      (Collision|SetCollisionResponsetoChannel (Variables|Default|GetMesh) "ECC_Visibility" "ECR_Block")
      (else
        (return)))
    (elif (<= Fade 0.0)
      (Collision|SetCollisionResponsetoChannel (Variables|Default|GetMesh) "ECC_Visibility" "ECR_Ignore")
      (else
        (return))))
  (return))