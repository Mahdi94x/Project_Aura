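; Flame pillar actor that flickers its fire light by varying the light's intensity.
; On BeginPlay it randomly picks one of two intensity timelines, and each picks again at random when it finishes, creating a continuous, varied loop.
; Timeline updates feed ScaleFlameIntensity, which multiplies the curve value by a base intensity and applies it to the light if valid.
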(event Custom|StartTimeLine_1
  (bind _flameintensity (Timeline|FlameIntensity_1 PlayFromStart)
    (:Update
      (CallFunction|ScaleFlameIntensity _flameintensity))
    (:Finished
      (CallFunction|ChooseTimeline))))

(event Custom|Start%20TimeLine_2
  (bind _flameintensity_2 (Timeline|FlameIntensity_2 PlayFromStart)
    (:Update
      (CallFunction|ScaleFlameIntensity _flameintensity_2))
    (:Finished
      (CallFunction|ChooseTimeline))))

(event Custom|ChooseTimeline
  (switch int (Math|Random|RandomIntegerinRange 0 1)
    (:Default
      (CallFunction|StartTimeLine2 :!label _label))
    (:0
      (CallFunction|StartTimeLine1))
    (:1
      (goto _label))))

(event EventBeginPlay
  (CallFunction|ChooseTimeline))

(fn ConstructionScript)

(fn ScaleFlameIntensity
  (params (Intensity :type Float%20%28double-precision%29))
  (bind _firelight (Variables|Default|GetFireLight)
    (:then
      (Rendering|Components|Light|SetIntensity _firelight (* Intensity (Variables|Default|GetBaseIntensity))))
    (:else)))