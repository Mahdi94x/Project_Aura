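; Behavior tree service that keeps an AI pawn's blackboard updated with the nearest opposing actor.
; Each tick it picks the target tag from the controlled pawn's own tag, so Player-tagged pawns seek Enemy actors and all others seek Player actors.
; It then linearly scans every actor with that tag and writes the closest one and its distance to blackboard keys.
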(event EventReceiveTickAI
  (params (OwnerController :type AI%20Controller%20Object%20Reference) (ControlledPawn :type Pawn%20Object%20Reference) (DeltaSeconds :type Float%20%28single-precision%29))
  (CallFunction|SetTargetTag ControlledPawn)
  (CallFunction|FindNearestPlayer ControlledPawn))

(fn SetTargetTag
  (params (ControlledPawn :type Actor%20Object%20Reference))
  (if (Actor|ActorHasTag ControlledPawn "Player")
    (Variables|Default|SetTargetTag "Enemy")
    (else
      (Variables|Default|SetTargetTag "Player"))))

(fn FindNearestPlayer
  (params (ControlledPawn :type Pawn%20Object%20Reference))
  (LocalVariables|SetClosestActor 0)
  (LocalVariables|SetClosestDistance 9999999999999.0)
  (bind _outactors (Actor|GetAllActorswithTag (Variables|Default|GetTargetTag)))
  (for _array_element _outactors
    (Utilities|IsValid _array_element
      (:Is%20Valid
        (Utilities|IsValid ControlledPawn
          (:Is%20Valid
            (bind _output_get (LocalVariables|SetActorFromArray _array_element))
            (bind _output_get_2 (LocalVariables|SetCalculatedDistance (Transformation|GetDistanceTo _output_get ControlledPawn)))
            (if (< _output_get_2 (LocalVariables|GetClosestDistance))
              (LocalVariables|SetClosestDistance (LocalVariables|GetCalculatedDistance))
              (LocalVariables|SetClosestActor (LocalVariables|GetActorFromArray))))))))
  (Class|BTFunctionLibrary|SetBlackboardValueasObject (Variables|Default|GetTargetToFollow_Selector) (LocalVariables|GetClosestActor))
  (Class|BTFunctionLibrary|SetBlackboardValueasFloat (Variables|Default|GetDistanceToTarget_Selector) (LocalVariables|GetClosestDistance)))